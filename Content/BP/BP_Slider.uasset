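; BP_Slider is a slide actor that tells overlapping actors to start sliding between two points.
; When its Collider begins an overlap, it sends StartSlidingMessage to the other actor with itself and the world locations of StartSocket and EndSocket.
; End overlap sends the same message and endpoints but leaves the Slider reference empty, leaving the response to the receiving actor.
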(event `self.collider.OnComponentBeginOverlap`
  (params (OverlappedComponent :type "PrimitiveComponent Object Reference") (OtherActor :type "Actor Object Reference") (OtherComp :type "PrimitiveComponent Object Reference") (OtherBodyIndex :type Integer) (bFromSweep :type Boolean) (SweepResult :type "HitResult Structure (by ref)"))
  (message `/Game/BP/BPI_Sliding.startSliding` OtherActor self (`SceneComponent.K2_GetComponentLocation` (`self.startSocket`)) (`SceneComponent.K2_GetComponentLocation` (`self.endSocket`))))

(event `self.collider.OnComponentEndOverlap`
  (params (OverlappedComponent :type "PrimitiveComponent Object Reference") (OtherActor :type "Actor Object Reference") (OtherComp :type "PrimitiveComponent Object Reference") (OtherBodyIndex :type Integer))
  (message `/Game/BP/BPI_Sliding.startSliding` OtherActor null (`SceneComponent.K2_GetComponentLocation` (`self.startSocket`)) (`SceneComponent.K2_GetComponentLocation` (`self.endSocket`))))

(fn `UserConstructionScript`)